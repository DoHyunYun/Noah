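; BP_Date is a map environment actor that runs a looping day and night cycle.
; Each Tick accumulates elapsed time and rotates SunLight, turning yaw a full circle per DayDuration while pitch follows a sine wave scaled by MaxSunHeight.
; It then refreshes BP_Sky_Sphere's sun direction and uses its SunHeight to switch the sky light color to black at or below the horizon, white above.
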(event `self.ReceiveTick`
  (params (DeltaSeconds :type "Float (single-precision)"))
  (set `self.SunDrive` (+ DeltaSeconds (`self.SunDrive`)))
  (`self.K2_SetActorRotation` (`self.SunLight`) (`KismetMathLibrary.MakeRotator` 0.0 (* (`KismetMathLibrary.Sin` (`KismetMathLibrary.MultiplyByPi` (* (/ (`self.SunDrive`) (`self.DayDuration`)) 2.0))) (`self.MaxSunHeight`)) (/ (* (`self.SunDrive`) 360.0) (`self.DayDuration`))) false)
  (bind _assky_light (cast `SkyLight` (`self.AmbLight`)))
  (bind _asbp_sky_sphere (cast `/Engine/EngineSky/BP_Sky_Sphere` (`self.SkySphere`)))
  (`/Engine/EngineSky/BP_Sky_Sphere.UpdateSunDirection` _asbp_sky_sphere)
  (if (<= (`/Engine/EngineSky/BP_Sky_Sphere.Sun height` _asbp_sky_sphere) 0.0)
    (`SkyLightComponent.SetLightColor` :`self` (`SkyLight.LightComponent` _assky_light))
    (else
      (`SkyLightComponent.SetLightColor` (`SkyLight.LightComponent` _assky_light) (struct :`R` 1.0 :`G` 1.0 :`B` 1.0 :`A` 1.0)))))

(fn `UserConstructionScript`)