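; BP_Stone is a damageable stone that drops its stored item when destroyed.
; BeginPlay initialises its child-actor Item with a random quantity and adds it to Inventory.
; DamagedandDeath plays a sound and either starts a shake, which Tick drives by jittering X/Y on a per-frame countdown, or handles death.
; On death, one spawned Item is re-initialised for each inventory entry until an empty code, then the stone is destroyed.
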(event `self.ReceiveBeginPlay`
  (bind _asitem (cast `Item` (`ChildActorComponent.ChildActor` (`self.ChildActor`))))
  (bind _returnvalue (`Item.InitItem` _asitem 1 (`KismetMathLibrary.RandomIntegerInRange` 1 10)))
  (`Inventory.AddItem` (`self.Inventory`) _returnvalue))

(event `self.ReceiveTick`
  (params (DeltaSeconds :type "Float (single-precision)"))
  (if (`self.IsDamaged`)
    (if (<= (`self.ShakeTime`) 0.0)
      (set `self.IsDamaged` false)
      (`self.K2_SetActorLocation` (`self.PreLocation`))
      (set `self.ShakeTime` 0.5)
      (else
        (`self.K2_SetActorLocation` (`KismetMathLibrary.MakeVector` (+ (.x (`self.PreLocation`)) (`KismetMathLibrary.RandomFloatInRange` -5.0 5.0)) (+ (.y (`self.PreLocation`)) (`KismetMathLibrary.RandomFloatInRange` -5.0 5.0)) (.z (`self.PreLocation`))))
        (set `self.ShakeTime` (- (`self.ShakeTime`) 0.05))))))

(fn `DamagedandDeath`
  (params (Damage :type Integer))
  (bind _returnvalue (`self.Damaged` Damage))
  (`GameplayStatics.PlaySoundAtLocation` "/Game/Resource/Sound/AttackTree.AttackTree" (`self.K2_GetActorLocation`))
  (if (<= _returnvalue 0)
    (bind _returnvalue_2 (`|SpawnActorFromClass` "/Script/Noah.Item" (`self.GetTransform`) "Undefined" "OverrideRootScale"))
    (for _array_element (`Inventory.ItemList` (`self.Inventory`))
      (bind _itemcode (`Item.ItemCode` _array_element))
      (if (<= _itemcode 0)
        (break)
        (else
          (bind _returnvalue_3 (`Item.InitItem` _returnvalue_2 _itemcode (`Item.Number` _array_element)))
          (`Item.SetMesh` _returnvalue_3))))
    (`self.K2_DestroyActor`)
    (else
      (set `self.isDamaged` true)
      (set `self.PreLocation` (`self.K2_GetActorLocation`)))))

(fn `UserConstructionScript`)