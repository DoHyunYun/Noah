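; BP_NoahCharacter is a player character Blueprint that plays an attack montage and picks up nearby items.
; JoinCollision overlaps register and unregister Items through DetectObject and MissObject, printing an error if removal fails.
; Pressing E, bound as a raw key, takes the result of FindNearItem, adds it to the inventory UI reached through BP_NoahHUD, then destroys the actor.
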(event `self.ReceiveBeginPlay`
  (`parent.ReceiveBeginPlay`))

(event `self.ReceiveTick`
  (params (DeltaSeconds :type "Float (single-precision)"))
  (`parent.ReceiveTick` DeltaSeconds))

(event `InputAction|Attack`
  (params (Key :type "Key Structure" :default "AnyKey"))
  (:`Pressed`
    (`AnimInstance.Montage_Play` (`SkeletalMeshComponent.GetAnimInstance` (`self.Mesh`)) "/Game/Character/Animation/Montage_Attack.Montage_Attack" 1.0 "MontageLength" 0.0)))

(event `self.JoinCollision.OnComponentBeginOverlap`
  (params (OverlappedComponent :type "PrimitiveComponent Object Reference") (OtherActor :type "Actor Object Reference") (OtherComp :type "PrimitiveComponent Object Reference") (OtherBodyIndex :type Integer) (bFromSweep :type Boolean) (SweepResult :type "HitResult Structure (by ref)"))
  ;[1 1 1] Detected Item
  (bind _asitem (cast `Item` OtherActor))
  (`self.DetectObject` _asitem))

(event `self.JoinCollision.OnComponentEndOverlap`
  (params (OverlappedComponent :type "PrimitiveComponent Object Reference") (OtherActor :type "Actor Object Reference") (OtherComp :type "PrimitiveComponent Object Reference") (OtherBodyIndex :type Integer))
  ;[1 1 1] Miss Item
  (bind _asitem (cast `Item` OtherActor))
  (bind _returnvalue (`self.MissObject` _asitem))
  (if (not _returnvalue)
    (`KismetSystemLibrary.PrintString` "Is serious missObject Error from BP_NoahCharacter")))

(event `Key|E`
  (params (Key :type "Key Structure" :default "AnyKey"))
  ;[1 1 1] Get Item
  (:`Pressed`
    (bind _returnvalue (`self.FindNearItem`))
    (bind _asitem (cast `Item` _returnvalue))
    (bind _asbp_noah_hud (cast `/Game/GameMode/BP_NoahHUD` (`PlayerController.GetHUD` (`GameplayStatics.GetPlayerController` 0))))
    (`/Game/UI/Inventory/Inventory.AddItem` (`/Game/UI/PlayerDefaultUI.InventoryUI` (`/Game/GameMode/BP_NoahHUD.PlayerDefaultUI` _asbp_noah_hud)) _asitem)
    (`self.K2_DestroyActor` _returnvalue)))

(fn `UserConstructionScript`
  (`parent.UserConstructionScript`))