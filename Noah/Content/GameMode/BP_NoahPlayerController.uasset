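; Player controller that handles inventory UI input and starts play in game-only input mode.
; The I key toggles the info UI on the player's default UI, switching input mode and mouse cursor to match.
; The L key is a test hook that randomizes the code and count of a child-actor Item and adds it to the inventory UI.
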(event `self.ReceiveBeginPlay`
  (`WidgetBlueprintLibrary.SetInputMode_GameOnly` (`GameplayStatics.GetPlayerController` 0)))

(event `Key|I`
  (params (Key :type "Key Structure" :default "AnyKey"))
  (bind _returnvalue (`GameplayStatics.GetPlayerController` 0))
  (bind _playerdefultui (`self.PlayerDefultUI`))
  (:`Pressed`
    (if (`self.ActiveInventory`)
      ;[1 1 1] 인벤토리UI 숨기기
      (`/Game/UI/PlayerDefaultUI.InfoUISetHidden` _playerdefultui)
      (set `self.ActiveInventory` false)
      (`WidgetBlueprintLibrary.SetInputMode_GameOnly` _returnvalue)
      (set `self.bShowMouseCursor` false)
      (else
        ;[1 1 1] 인벤토리UI 표시
        (`/Game/UI/PlayerDefaultUI.InfoUISetVisible` _playerdefultui)
        (set `self.ActiveInventory` true)
        (`WidgetBlueprintLibrary.SetInputMode_GameAndUIEx` _returnvalue)
        (set `self.bShowMouseCursor` true)))))

(event `Key|L`
  (params (Key :type "Key Structure" :default "AnyKey"))
  (:`Pressed`
    ;[1 1 1] 아이템 추가
    (bind _asitem (cast `Item` (`ChildActorComponent.ChildActor` (`self.ChildActor`))))
    (set `Item.ItemCode` (`KismetMathLibrary.RandomIntegerInRange` 1 2) _asitem)
    (set `Item.Number` (`KismetMathLibrary.RandomIntegerInRange` 1 3) _asitem)
    (`/Game/UI/Inventory/Inventory.AddItem` (`/Game/UI/PlayerDefaultUI.InventoryUI` (`self.PlayerDefultUI`)) _asitem)))

(fn `UserConstructionScript`)