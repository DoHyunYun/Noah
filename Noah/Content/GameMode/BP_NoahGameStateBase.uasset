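; Game state Blueprint for the Noah game that tracks the passing days and the rising water level.
; On BeginPlay it caches the first BP_Wave actor found in the level.
; Each AddDay event increments the day count, adds a fixed amount to the accumulated rain value, and passes that total to the wave's UpWave.
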(event `self.ReceiveBeginPlay`
  (bind _outactors (`GameplayStatics.GetAllActorsOfClass` "/Game/MapEnvironment/BP_Wave.BP_Wave_C"))
  (set `self.Wave` (`KismetArrayLibrary.Array_Get` _outactors)))

(event `self.ReceiveTick`
  (params (DeltaSeconds :type "Float (single-precision)")))

(event `self.AddDay`
  (`/Engine/EditorBlueprintResources/StandardMacros.IncrementInt` (`self.Day`)
    (:`  `
      (bind _output_get (set `self.RainValue` (+ (`self.RainValue`) 20)))
      (`Wave.UpWave` (`self.Wave`) _output_get))))

(fn `UserConstructionScript`)