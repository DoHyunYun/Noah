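; Environment manager that runs the day/night cycle and rain weather for the level.
; Tick advances a time value to rotate the sun, drives light intensity, sky and cloud colors from curves keyed on sun height, then refreshes BP_SkySphere.
; At day's end it resets the clock and increments the day in the game state.
; RainValue darkens sky and lights, and scales a player-following rain emitter once it reaches half.
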(event `self.ReceiveBeginPlay`
  (bind _asbp_sky_sphere (cast `/Game/MapEnvironment/BP_SkySphere` (`self.SkySphere`)))
  (set `self.ReSkySphere` _asbp_sky_sphere)
  (bind _returnvalue (`GameplayStatics.SpawnEmitterAtLocation` "/Game/Resource/Particle/P_Rainfall.P_Rainfall" (`self.K2_GetActorLocation` (`GameplayStatics.GetPlayerPawn` 0))))
  (set `self.RainParticle` _returnvalue))

(event `self.ReceiveTick`
  (params (DeltaSeconds :type "Float (single-precision)"))
  (bind _returnvalue (`CurveLinearColor.GetLinearColorValue` (`self.CurveSkyLightColor`) (`/Game/MapEnvironment/BP_SkySphere.Sun height` (`self.ReSkySphere`))))
  (set `self.SunDrive` (+ DeltaSeconds (`self.SunDrive`)))
  (`|ExecutionSequence`
    (:`then_0`
      ;[1 1 1] 해 위치(회전) 계산
      (bind _returnvalue_2 (`self.SeekSunRotator` (`self.SunDrive`) (`self.DayDuration`) (`self.MaxSunHeight`)))
      (`self.K2_SetActorRotation` (`self.DirectionLight`) _returnvalue_2 false))
    (:`then_1`
      ;[1 1 1] 해의 위치에 따른 이벤트 발생
      (if (>= (`self.SunDrive`) (`self.DayDuration`))
        (`self.Tomorrow`))
      (`LightComponent.SetIntensity` (`Light.LightComponent` (`self.DirectionLight`)) (`CurveFloat.GetFloatValue` (`self.CurveSunIntensity`) (`/Game/MapEnvironment/BP_SkySphere.Sun height` (`self.ReSkySphere`)))))
    (:`then_2`
      ;[1 1 1] 해 높이에 따른 SkyLight의 색 조정
      (`SkyLightComponent.SetLightColor` (`SkyLight.LightComponent` (`self.SkyLight`)) _returnvalue)
      (set `/Game/MapEnvironment/BP_SkySphere.Cloud color` _returnvalue (`self.ReSkySphere`)))
    (:`then_3`
      ;[1 1 1] 비의 양에 따른 날씨 효과 설정
      (`self.Rain` (`self.RainValue`))
      ;[1 1 1] 해의 정보 갱신
      (`/Game/MapEnvironment/BP_SkySphere.UpdateSkySphere` (`self.ReSkySphere`)))))

(event `self.Tomorrow`
  (set `self.SunDrive` 0.0)
  (bind _asbp_noah_game_state_base (cast `/Game/GameMode/BP_NoahGameStateBase` (`GameplayStatics.GetGameState`)))
  (`NoahGameStateBase.AddDay` _asbp_noah_game_state_base))

(event `Rain`
  (params (value :type "Float (double-precision)"))
  (`self.UpdateRain` value)
  (`self.UpdateRainSky` value))

(fn `UpdateRain`
  (params (Value :type "Float (double-precision)"))
  ;[1 1 1] 플레이어를 따라다니며 주변에만 비가 오도록 설정.
  (`SceneComponent.K2_SetWorldLocation` (`self.RainParticle`) (`self.K2_GetActorLocation` (`GameplayStatics.GetPlayerPawn` 0)) false false)
  ;[1 1 1] 강수량이 0.5이상이라면 비가 내리기 시작한다.
  (if (< Value 0.5)
    (`ParticleSystemComponent.SetFloatParameter` (`self.RainParticle`) "RainNumber" 0.0)
    (else
      (`ParticleSystemComponent.SetFloatParameter` (`self.RainParticle`) "RainNumber" (`KismetMathLibrary.Lerp` 50000.0 630000.0 (* (- Value 0.5) 2.0))))))

(fn `UpdateRainSky`
  (params (Value :type "Float (double-precision)"))
  (locals (InvValue :type "Float (double-precision)") (ReValue :type "Float (double-precision)"))
  (bind _reskysphere (`self.ReSkySphere`))
  (bind _reskysphere_2 (`self.ReSkySphere`))
  (bind _reskysphere_3 (`self.ReSkySphere`))
  (bind _lightcomponent (`Light.LightComponent` (`self.DirectionLight`)))
  (set `local.ReValue` Value)
  (set `local.InvValue` (- 1.0 Value))
  (`|ExecutionSequence`
    (:`then_0`
      ;[0.595 0.3649 0.09635] 강수량에 따른 SkySphere, DirectionLight, SkyLight 색을 조정해준다.
      ;;[1 1 1] 해의 밝기
      (`LightComponent.SetIntensity` _lightcomponent (* (`local.InvValue`) (`LightComponentBase.Intensity` _lightcomponent)))
      ;;[1 1 1] 태양의 투명도
      (set `/Game/MapEnvironment/BP_SkySphere.Sun brightness` (`local.InvValue`) (`self.ReSkySphere`))
      ;;[1 1 1] 구름 색
      (set `/Game/MapEnvironment/BP_SkySphere.Cloud color` (* (`/Game/MapEnvironment/BP_SkySphere.Cloud color` _reskysphere) (`local.InvValue`)) _reskysphere)
      ;;[1 1 1] 구름 투명도
      (set `/Game/MapEnvironment/BP_SkySphere.Cloud opacity` (`KismetMathLibrary.Lerp` 1.0 2.0 (`local.ReValue`)) (`self.ReSkySphere`)))
    (:`then_1`
      ;;[1 1 1] 수평선 색
      (set `/Game/MapEnvironment/BP_SkySphere.Horizon color` (* (`CurveLinearColor.GetLinearColorValue` (`self.CurveHorizonColor`) (`/Game/MapEnvironment/BP_SkySphere.Sun height` _reskysphere_2)) (`KismetMathLibrary.LinearColorLerp` (struct :`R` 1.0 :`G` 1.0 :`B` 1.0 :`A` 1.0) (struct :`A` 1.0) (`local.ReValue`))) _reskysphere_2)
      ;;[1 1 1] 하늘 위(천정) 색
      (set `/Game/MapEnvironment/BP_SkySphere.Zenith Color` (* (`CurveLinearColor.GetLinearColorValue` (`self.CurveZenithColor`) (`/Game/MapEnvironment/BP_SkySphere.Sun height` _reskysphere_3)) (`KismetMathLibrary.LinearColorLerp` (struct :`R` 1.0 :`G` 1.0 :`B` 1.0 :`A` 1.0) (struct :`A` 1.0) (`local.ReValue`))) _reskysphere_3)
      ;;[1 1 1] 종합적인 색
      (set `/Game/MapEnvironment/BP_SkySphere.Overall Color` (`CurveLinearColor.GetLinearColorValue` (`self.CurveOverallColor`) (`local.ReValue`)) (`self.ReSkySphere`))
      ;;[1 1 1] 주변광(SkyLight) 색
      (`SkyLightComponent.SetLightColor` (`SkyLight.LightComponent` (`self.SkyLight`)) (* (`LightComponentBase.GetLightColor` (`SkyLight.LightComponent` (`self.SkyLight`))) (`local.InvValue`))))))

(fn `UserConstructionScript`)