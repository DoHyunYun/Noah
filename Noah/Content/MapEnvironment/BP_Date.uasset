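; BP_Date runs the day-night cycle and advances the game's day count.
; Tick accumulates SunDrive time, rotates the directional light through SeekSunRotator, tints the SkyLight from a color curve keyed on BP_Sky_Sphere's SunHeight, and refreshes the sky sphere.
; It sets sunlight intensity every tick, on for the first half of DayDuration and off for the second.
; When DayDuration is reached, SunDrive resets and BP_NoahGameStateBase adds a day.
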(event `self.ReceiveTick`
  (params (DeltaSeconds :type "Float (single-precision)"))
  (bind _dayduration (`self.DayDuration`))
  (set `self.SunDrive` (+ DeltaSeconds (`self.SunDrive`)))
  (`|ExecutionSequence`
    (:`then_0`
      ;[1 1 1] 해 위치(회전) 계산
      (bind _returnvalue (`self.SeekSunRotator` (`self.SunDrive`) (`self.DayDuration`) (`self.MaxSunHeight`)))
      (`self.K2_SetActorRotation` (`self.DirectionLight`) _returnvalue false))
    (:`then_1`
      ;[1 1 1] 해의 위치에 따른 이벤트 발생
      (if (>= (`self.SunDrive`) _dayduration)
        (`self.Tomorrow`)
        (elif (>= (/ _dayduration 2.0) (`self.SunDrive`))
          (`self.SunUp`)
          (else
            (`self.SunDown`)))))
    (:`then_2`
      ;[1 1 1] SkyLight의 색 조정
      (bind _asbp_sky_sphere (cast `/Engine/EngineSky/BP_Sky_Sphere` (`self.SkySphere`)))
      (`SkyLightComponent.SetLightColor` (`SkyLight.LightComponent` (`self.SkyLight`)) (`CurveLinearColor.GetLinearColorValue` (`self.CurveAmbColor`) (`/Engine/EngineSky/BP_Sky_Sphere.Sun height` _asbp_sky_sphere)))
      ;[1 1 1] 해의 정보 갱신
      (bind _asbp_sky_sphere_2 (cast `/Engine/EngineSky/BP_Sky_Sphere` (`self.SkySphere`)))
      (`/Engine/EngineSky/BP_Sky_Sphere.UpdateSunDirection` _asbp_sky_sphere_2))))

(event `self.Tomorrow`
  (set `self.SunDrive` 0.0)
  (bind _asbp_noah_game_state_base (cast `/Game/GameMode/BP_NoahGameStateBase` (`GameplayStatics.GetGameState`)))
  (`NoahGameStateBase.AddDay` _asbp_noah_game_state_base))

(event `self.SunUp`
  (`LightComponent.SetIntensity` (`Light.LightComponent` (`self.DirectionLight`)) 3.0))

(event `self.SunDown`
  (`LightComponent.SetIntensity` (`Light.LightComponent` (`self.DirectionLight`)) 0.0))

(fn `UserConstructionScript`)