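; BP_Wave is a water surface actor that can rise and applies an underwater look when the player's camera is below it.
; The UpWave event offsets the wave mesh upward in world Z by the supplied rain value.
; Each Tick compares BP_NoahCharacter's follow camera height with the mesh, setting a cyan post-process color and blendable material when submerged.
; Above water, it sets white and makes a zero-weight blendable call without specifying the material.
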(event `self.ReceiveBeginPlay`)

(event `self.UpWave`
  (params (RainValue :type Integer))
  (`SceneComponent.K2_AddWorldOffset` (`self.WaveMeshComponent`) (`KismetMathLibrary.MakeVector` 0.0 0.0 (`KismetMathLibrary.Conv_IntToDouble` RainValue)) false false))

(event `self.ReceiveTick`
  (params (DeltaSeconds :type "Float (single-precision)"))
  (bind _postprocess (`self.PostProcess`))
  (bind _postprocess_2 (`self.PostProcess`))
  (bind _asbp_noah_character (cast `/Game/GameMode/BP_NoahCharacter` (`GameplayStatics.GetPlayerPawn` 0)))
  (if (<= (.z (`SceneComponent.K2_GetComponentLocation` (`NoahCharacter.FollowCamera` _asbp_noah_character))) (.z (`SceneComponent.K2_GetComponentLocation` (`self.WaveMeshComponent`))))
    (set `PostProcessComponent.Settings` (make `PostProcessSettings` :`SceneColorTint` (struct :`R` 0.425 :`G` 0.9466 :`B` 1.0 :`A` 1.0)) _postprocess)
    (`PostProcessComponent.AddOrUpdateBlendable` _postprocess (`self.Material`) 1.0)
    (else
      (set `PostProcessComponent.Settings` (make `PostProcessSettings`) _postprocess_2)
      (`PostProcessComponent.AddOrUpdateBlendable` _postprocess_2 null 0.0))))

(fn `UserConstructionScript`)